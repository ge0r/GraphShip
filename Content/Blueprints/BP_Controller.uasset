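; BP_Controller turns player turn inputs into direction change requests for the spaceship.
; On BeginPlay it finds and caches the BP_SpaceShip actor, then each Left, Right, Up or Down press prints a label and calls RequestDirectionChange with an axis unit vector.
; PageUp and PageDown speed up or slow game time through slomo console commands.
; SetDirection is an empty stub.
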(event `Detect SpaceShip`
  (bind _returnvalue (`GameplayStatics.GetActorOfClass` "/Game/Blueprints/BP_SpaceShip.BP_SpaceShip_C"))
  (set `self.SpaceShip` _returnvalue))

(event `self.ReceiveBeginPlay`
  (`self.Detect SpaceShip`))

(event `InputAction|LeftTurn`
  (params (Key :type "Key Structure"))
  ;[1 1 1] Controls
  (:`Pressed`
    (`KismetSystemLibrary.PrintString` "Left")
    (`SpaceShip.RequestDirectionChange` (`self.SpaceShip`) (0.0 -1.0 0.0))))

(event `InputAction|RightTurn`
  (params (Key :type "Key Structure"))
  ;[1 1 1] Controls
  (:`Pressed`
    (`KismetSystemLibrary.PrintString` "Right")
    (`SpaceShip.RequestDirectionChange` (`self.SpaceShip`) (0.0 1.0 0.0))))

(event `InputAction|UpTurn`
  (params (Key :type "Key Structure"))
  ;[1 1 1] Controls
  (:`Pressed`
    (`KismetSystemLibrary.PrintString` "Up")
    (`SpaceShip.RequestDirectionChange` (`self.SpaceShip`) (1.0 0.0 0.0))))

(event `InputAction|DownTurn`
  (params (Key :type "Key Structure"))
  ;[1 1 1] Controls
  (:`Pressed`
    (`KismetSystemLibrary.PrintString` "Down")
    (`SpaceShip.RequestDirectionChange` (`self.SpaceShip`) (-1.0 0.0 0.0))))

(event `Key|PageUp`
  (params (Key :type "Key Structure"))
  (:`Pressed`
    (`KismetSystemLibrary.ExecuteConsoleCommand` "slomo 5" null)))

(event `Key|PageDown`
  (params (Key :type "Key Structure"))
  (:`Pressed`
    (`KismetSystemLibrary.ExecuteConsoleCommand` "slomo 0.1" null)))

(fn `SetDirection`
  (params (Direction :type "Vector Structure")))

(fn `UserConstructionScript`)